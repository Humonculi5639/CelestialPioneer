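; Test Blueprint that drives a static mesh with tank-style controls from axis input.
; Left_Right steps a stored Direction yaw by RotationSpeed and sets the mesh's world rotation to it.
; Forward_Back builds a Speed-scaled vector along that yaw with cosine and sine, negated for backward input, and applies it as a physics force.
; Axis values are used only for their sign, and nothing scales by delta time.
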(event Collision|EventActorBeginOverlap
  (params (OtherActor :type Actor%20Object%20Reference)))

(event EventTick
  (params (DeltaSeconds :type Float%20%28single-precision%29)))

(event Input|AxisEvents|InputAxisForward_Back
  (params (AxisValue :type Float%20%28single-precision%29))
  (bind _speed (Variables|Default|GetSpeed))
  (bind _direction (Variables|Default|GetDirection))
  (bind _returnvalue (Math|Conversions|ToFloat(Integer) _direction))
  (bind _returnvalue_2 (Math|Conversions|ToFloat(Integer) _speed))
  (bind _returnvalue_3 (Math|Trig|Cos(Degrees) _returnvalue))
  (bind _returnvalue_4 (Math|Trig|Sin(Degrees) _returnvalue))
  (bind _returnvalue_5 (* _returnvalue_2 _returnvalue_4))
  (bind _returnvalue_6 (* _returnvalue_2 _returnvalue_3))
  (bind _returnvalue_7 (Math|Vector|MakeVector _returnvalue_6 _returnvalue_5 0.0))
  (if (> AxisValue 0.0) ; if positive
    (Variables|Default|SetMovement _returnvalue_7)
    (Physics|AddForce (Variables|Debug|GetStaticMeshComponent) (Variables|Default|GetMovement) "None" false :!label _label)
    (elif (> 0.0 AxisValue) ; if negative
      (Variables|Default|SetMovement (* _returnvalue_7 -1))
      (goto _label))))

(event Input|AxisEvents|InputAxisLeft_Right
  (params (AxisValue :type Float%20%28single-precision%29))
  (if (> AxisValue 0.0) ; if positive
    (Variables|Default|SetDirection (+ (Variables|Default|GetDirection) (Variables|Default|GetRotation%20Speed)))
    (Transformation|SetWorldRotation (Variables|Debug|GetStaticMeshComponent) (Math|Rotator|MakeRotator 0.0 0.0 (Math|Conversions|ToFloat(Integer) (Variables|Default|GetDirection))) false false :!label _label)
    (elif (> 0.0 AxisValue) ; if negative
      (Variables|Default|SetDirection (- (Variables|Default|GetDirection) (Variables|Default|GetRotation%20Speed)))
      (goto _label))))

(fn ConstructionScript)