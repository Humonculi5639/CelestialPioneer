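; Bullet Blueprint that moves a physics component with a constant force along world X, applied every tick.
; The Left_Right input axis steers it: negative values apply a large negative yaw torque scaled by the Rot variable.
; Positive axis values do nothing, as the opposite torque node is left unconnected.
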(event EventTick
  (params (DeltaSeconds :type Float%20%28single-precision%29))
  (Physics|AddForce (Variables|Default|GetBullet) "100.000000, 0, 0" "None" false))

(event Input|AxisEvents|InputAxisLeft_Right
  (params (AxisValue :type Float%20%28single-precision%29))
  (if (not (> AxisValue 0.0))
    (if (> 0.0 AxisValue)
      (Class|PrimitiveComponent|AddTorqueinDegrees (Variables|Default|GetBullet) (* (Math|Vector|MakeVector 0.0 0.0 (Math|Conversions|ToFloat(Integer) (Variables|Default|GetRot))) -1000000) "None" false))))

(fn ConstructionScript)