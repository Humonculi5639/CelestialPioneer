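; SpaceSkybox_Bp is a space skybox actor that configures a static mesh as the sky backdrop.
; Its construction script disables mesh collision, sets shadow casting from a variable and applies the chosen material.
; It writes star brightness, scene brightness and power into the SpaceSkybox_Params Material Parameter Collection, so those values are global to materials reading it rather than per instance.
; The event graph holds no active logic.
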(event EventBeginPlay)

(event Collision|EventActorBeginOverlap
  (params (OtherActor :type Actor%20Object%20Reference)))

(event EventTick
  (params (DeltaSeconds :type Float%20%28single-precision%29)))

(fn ConstructionScript
  (Collision|SetCollisionEnabled (Variables|Default|GetStaticMesh) "NoCollision")
  (Rendering|SetCastShadow (Variables|Default|GetStaticMesh) (Variables|Default|GetCast%20Shadow))
  (Rendering|Material|SetMaterial (Variables|Default|GetStaticMesh) 0 (Variables|Default|GetMaterial))
  (Rendering|Material|SetScalarParameterValue "/Game/Blueprints/SpaceSkybox_Params.SpaceSkybox_Params" "Star Brightness" (Variables|Default|GetStar%20Brightness) :!class /Script/Engine.KismetMaterialLibrary)
  (Rendering|Material|SetScalarParameterValue "/Game/Blueprints/SpaceSkybox_Params.SpaceSkybox_Params" "Scene Brightness" (Variables|Default|GetScene%20Brightness) :!class /Script/Engine.KismetMaterialLibrary)
  (Rendering|Material|SetScalarParameterValue "/Game/Blueprints/SpaceSkybox_Params.SpaceSkybox_Params" "Power" (Variables|Default|GetPower) :!class /Script/Engine.KismetMaterialLibrary))