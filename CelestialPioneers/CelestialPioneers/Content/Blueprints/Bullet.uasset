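; Bullet actor that serves as either a player or enemy projectile, set by the PlayerBullet flag.
; On hit, enemy bullets decrement the health of the MovementTest player stored in SpaceGameInstance, while player bullets destroy EnemyShip actors.
; Both valid hits destroy the bullet, and other hits leave it alive.
; A Tick counter also destroys it after a fixed number of frames, so lifetime depends on frame rate.
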(event EventBeginPlay)

(event EventTick
  (params (DeltaSeconds :type Float%20%28single-precision%29))
  (bind _timer (Variables|Default|Gettimer))
  (Math|Integer|IncrementInt _timer
    (:%20%20
      (if (>= _timer 60)
        (Actor|DestroyActor)))))

(event Collision|EventHit
  (params (MyComp :type Primitive%20Component%20Object%20Reference) (Other :type Actor%20Object%20Reference) (OtherComp :type Primitive%20Component%20Object%20Reference) (bSelfMoved :type Boolean) (HitLocation :type Vector :default "0, 0, 0") (HitNormal :type Vector :default "0, 0, 0") (NormalImpulse :type Vector :default "0, 0, 0") (Hit :type Hit%20Result%20Structure%20%28by%20ref%29))
  (bind _returnvalue (Utilities|GetClass Other))
  (bind _asspace_game_instance (Utilities|Casting|CastToSpaceGameInstance (Game|GetGameInstance)))
  (bind _asmovement_test (Utilities|Casting|CastToMovementTest (Variables|/Game/Blueprints/SpaceGameInstance.SpaceGameInstance_C|GetPlayer%20Actor _asspace_game_instance))
    (:then
      _)
    (:CastFailed
      _))
  (if (and (== _returnvalue "/Game/MovementTest.MovementTest_C") (not (Variables|Default|GetPlayerBullet)))
    (Default|DecrementHealth _asmovement_test)
    (Actor|DestroyActor :!label _label)
    (elif (and (== _returnvalue "/Game/EnemyShip.EnemyShip_C") (Variables|Default|GetPlayerBullet))
      (Actor|DestroyActor Other)
      (goto _label))))

(fn ConstructionScript)

(fn GetPlayerBullet
  (return (Variables|Default|GetPlayerBullet)))

(fn SetPlayerBullet
  (params (bool :type Boolean))
  (Variables|Default|SetPlayerBullet bool))